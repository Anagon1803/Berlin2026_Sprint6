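; BPC_VariableLight is a component that continuously varies the intensity of a referenced light in a wavering pulse.
; Each Tick adds or subtracts a fixed amount, flipping direction when a step counter reaches the current limit.
; Uneven up and down step limits make intensity drift in a zigzag, and Switch swaps them at the min/max intensity bounds to reverse the drift.
; Timing counts frames, so speed depends on frame rate.
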(event Custom|DecreaseLight
  (Variables|Default|SetIntensity (- (Variables|Default|GetIntensity) (Variables|Default|GetValeur)))
  (Rendering|Components|Light|SetIntensity (Variables|Default|GetLightRef) (Variables|Default|GetIntensity)))

(event Custom|IncreaseLight
  (Variables|Default|SetIntensity (+ (Variables|Default|GetIntensity) (Variables|Default|GetValeur)))
  (Rendering|Components|Light|SetIntensity (Variables|Default|GetLightRef) (Variables|Default|GetIntensity)))

(event Custom|Switch
  (if (>= (Variables|Default|GetIntensity) (Variables|Default|GetIntensityMax))
    (Variables|Default|SetMaximumLimit 15)
    (Variables|Default|SetMinimumLimit 20)
    (elif (<= (Variables|Default|GetIntensity) (Variables|Default|GetIntensityMin))
      (Variables|Default|SetMaximumLimit 20)
      (Variables|Default|SetMinimumLimit 15))))

(event EventBeginPlay
  (Variables|Default|SetMaximumLimit 20)
  (Variables|Default|SetMinimumLimit 15)
  (Variables|Default|SetIntensity (Variables|Default|GetIntensityMin)))

(event EventTick
  (params (DeltaSeconds :type Float%20%28single-precision%29))
  (if (Variables|Default|GetIndex)
    (CallFunction|IncreaseLight)
    (bind _return (CallFunction|IsMaximumStep?))
    (if _return
      (Variables|Default|SetIndex false)
      (Variables|Default|SetStep 0)
      (CallFunction|Switch)
      (else
        (Variables|Default|SetStep (+ (Variables|Default|GetStep) 1))))
    (else
      (CallFunction|DecreaseLight)
      (bind _return_2 (CallFunction|IsMinimumStep?))
      (if _return_2
        (Variables|Default|SetIndex true)
        (Variables|Default|SetStep 0)
        (CallFunction|Switch)
        (else
          (Variables|Default|SetStep (+ (Variables|Default|GetStep) 1)))))))

(fn IsMaximumStep?
  (return (== (Variables|Default|GetMaximumLimit) (Variables|Default|GetStep))))

(fn IsMinimumStep?
  (return (== (Variables|Default|GetMinimumLimit) (Variables|Default|GetStep))))